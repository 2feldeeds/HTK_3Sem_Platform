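; One-shot interactable button that plays the ShipGoesDown level sequence and then lets the player trigger the outside-spaceship transition.
; Interact plays a click, pushes the button via a timeline and starts the sequence after a delay.
; When the sequence finishes, it enables the SpawnBack volume, which calls OutsideSpaceShip on an overlapping BP_HtkCharacter.
; The E prompt shows while the character is inside the Sphere and turns toward the camera each tick.
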(event OnComponentBeginOverlap(Sphere)
  (params (OverlappedComponent :type Primitive%20Component%20Object%20Reference) (OtherActor :type Actor%20Object%20Reference) (OtherComp :type Primitive%20Component%20Object%20Reference) (OtherBodyIndex :type Integer) (bFromSweep :type Boolean) (SweepResult :type Hit%20Result%20Structure%20%28by%20ref%29))
  (Utilities|Casting|CastToBP_HtkCharacter OtherActor)
  (Rendering|SetVisibility (Variables|Default|GetE) true false))

(event OnComponentEndOverlap(Sphere)
  (params (OverlappedComponent :type Primitive%20Component%20Object%20Reference) (OtherActor :type Actor%20Object%20Reference) (OtherComp :type Primitive%20Component%20Object%20Reference) (OtherBodyIndex :type Integer))
  (Utilities|Casting|CastToBP_HtkCharacter OtherActor)
  (Rendering|SetVisibility (Variables|Default|GetE) false false))

(event OnComponentBeginOverlap(SpawnBack)
  (params (OverlappedComponent :type Primitive%20Component%20Object%20Reference) (OtherActor :type Actor%20Object%20Reference) (OtherComp :type Primitive%20Component%20Object%20Reference) (OtherBodyIndex :type Integer) (bFromSweep :type Boolean) (SweepResult :type Hit%20Result%20Structure%20%28by%20ref%29))
  (bind _asbp_htk_character (Utilities|Casting|CastToBP_HtkCharacter OtherActor))
  (Default|OutsideSpaceShip _asbp_htk_character))

(event Custom|Finished
  (Sequencer|Player|Stop (Variables|/Script/LevelSequence.LevelSequenceActor|GetSequencePlayer (stale EventInteract _outactor)) :!class /Script/MovieScene.MovieSceneSequencePlayer)
  (Collision|SetCollisionEnabled (Variables|Default|GetSpawnBack) "QueryOnly"))

(event EventTick
  (params (DeltaSeconds :type Float%20%28single-precision%29))
  (bind _e (Variables|Default|GetE))
  (Transformation|SetWorldRotation _e (Math|Rotator|FindLookatRotation (Transformation|GetWorldLocation _e) (Transformation|GetWorldLocation (Variables|/Script/Engine.Actor|GetRootComponent (Game|GetPlayerCameraManager 0)))) false false))

(event EventBeginPlay
  (Collision|SetCollisionEnabled (Variables|Default|GetSpawnBack) "NoCollision")
  (Rendering|SetVisibility (Variables|Default|GetE) false false))

(event EventInteract
  (Utilities|FlowControl|DoOnce false
    (:Completed
      (Audio|PlaySound2D "/Engine/VREditor/Sounds/UI/Click_on_Button.Click_on_Button" 1.0 1.0 0.0 0 0)
      (bind _button (Timeline|Timeline Play)
        (:Update
          (Transformation|AddRelativeLocation (Variables|Default|GetButton) (Math|Vector|MakeVector 0.0 0.0 (* _button (Variables|Default|GetButtonPush))) false false)
          (Utilities|FlowControl|Delay 3.0)
          (bind (_outactor _returnvalue) (Sequencer|Player|CreateLevelSequencePlayer "/Game/CutScene/ShipGoesDown.ShipGoesDown"))
          (Sequencer|Player|Play (Variables|/Script/LevelSequence.LevelSequenceActor|GetSequencePlayer _outactor) :!class /Script/MovieScene.MovieSceneSequencePlayer)
          (EventDispatchers|AssignOnFinished _returnvalue (delegate Custom|Finished)))))))

(fn ConstructionScript)