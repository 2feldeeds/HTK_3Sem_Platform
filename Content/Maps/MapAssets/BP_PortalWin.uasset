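; BP_PortalWin is a map actor that toggles a Portal component based on the state of five referenced buttons.
; Tick polls the StartCountDown flag on every button and, while all five are true, hides Portal and its child components.
; The check repeats each frame with no latch, and the Blueprint contains no logic to show Portal again or handle overlaps.
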(event EventBeginPlay)

(event Collision|EventActorBeginOverlap
  (params (OtherActor :type Actor%20Object%20Reference)))

(event EventTick
  (params (DeltaSeconds :type Float%20%28single-precision%29))
  (if (Math|Boolean|ANDBoolean (Variables|/Game/Maps/BP_OpenPortal.BP_OpenPortal_C|GetStartCountDown (Variables|Default|Getbutton)) (Variables|/Game/Maps/BP_OpenPortal.BP_OpenPortal_C|GetStartCountDown (Variables|Default|Getbutton_0)) (Variables|/Game/Maps/BP_OpenPortal.BP_OpenPortal_C|GetStartCountDown (Variables|Default|Getbutton_1)) (Variables|/Game/Maps/BP_OpenPortal.BP_OpenPortal_C|GetStartCountDown (Variables|Default|Getbutton_2)) (Variables|/Game/Maps/BP_OpenPortal.BP_OpenPortal_C|GetStartCountDown (Variables|Default|Getbutton_3)))
    (Rendering|SetVisibility (Variables|Default|GetPortal) false true)))

(fn ConstructionScript)