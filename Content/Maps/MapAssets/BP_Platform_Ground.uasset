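; BP_Platform_Ground is a map platform that moves up and down in an endless loop.
; On BeginPlay it sets a random yaw on its Scene component, then uses PlatformGroundType to run either the Begin Up or Begin Down graph.
; Each graph chains two timelines, one playing forward and one reversing from the end, scaling their output by Hight to drive the Scene's relative Z.
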(event Custom|DynamicMovement
  (switch Utilities|FlowControl|Switch|SwitchonEPlatformGroundType (Variables|Default|GetPlatformGroundType)
    (:NewEnumerator0
      (|BeginUp))
    (:NewEnumerator1
      (|BeginDown))))

(event EventBeginPlay
  (Transformation|SetRelativeRotation (Variables|Default|GetScene) (Math|Rotator|MakeRotator 0.0 0.0 (Math|Random|RandomFloatinRange -45.0 45.0)) false false)
  (CallFunction|DynamicMovement))

(event EventTick
  (params (DeltaSeconds :type Float%20%28single-precision%29)))

(fn ConstructionScript)