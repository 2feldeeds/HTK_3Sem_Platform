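; BP_Won is a level win trigger that sends the game to the Yoyo_Credits level.
; Overlap of its Sphere by BP_HtkCharacter sets a winning flag, which is never cleared.
; Tick polls that flag along with the IsDead state of six referenced enemies and opens the credits level once all are true.
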(event OnComponentBeginOverlap(Sphere)
  (params (OverlappedComponent :type Primitive%20Component%20Object%20Reference) (OtherActor :type Actor%20Object%20Reference) (OtherComp :type Primitive%20Component%20Object%20Reference) (OtherBodyIndex :type Integer) (bFromSweep :type Boolean) (SweepResult :type Hit%20Result%20Structure%20%28by%20ref%29))
  (Utilities|Casting|CastToBP_HtkCharacter OtherActor)
  (Variables|Default|SetIsWinng true))

(event EventBeginPlay)

(event Collision|EventActorBeginOverlap
  (params (OtherActor :type Actor%20Object%20Reference)))

(event EventTick
  (params (DeltaSeconds :type Float%20%28single-precision%29))
  (if (Math|Boolean|ANDBoolean (Variables|Default|GetIsWinng) (Variables|/Game/Enemy/BP_EnemyDefault.BP_EnemyDefault_C|GetIsDead (Variables|Default|GetEnemy1)) (Variables|/Game/Enemy/BP_EnemyDefault.BP_EnemyDefault_C|GetIsDead (Variables|Default|GetEnemy2)) (Variables|/Game/Enemy/BP_EnemyDefault.BP_EnemyDefault_C|GetIsDead (Variables|Default|GetEnemy3)) (Variables|/Game/Enemy/BP_EnemyDefault.BP_EnemyDefault_C|GetIsDead (Variables|Default|GetEnemy4)) (Variables|/Game/Enemy/BP_EnemyDefault.BP_EnemyDefault_C|GetIsDead (Variables|Default|GetEnemy5)) (Variables|/Game/Enemy/BP_EnemyDefault.BP_EnemyDefault_C|GetIsDead (Variables|Default|GetEnemy6)))
    (Game|OpenLevel(byObjectReference) "/Game/Maps/Yoyo_Credits.Yoyo_Credits")))

(fn ConstructionScript)