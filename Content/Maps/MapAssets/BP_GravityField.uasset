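; BP_GravityField is a map volume that inverts gravity for BP_HtkCharacter while it is inside the Box.
; Box overlap sets the movement component's gravity upward and flips the character's controls; leaving restores downward gravity and normal controls.
; Overlap also toggles PlaySound, which Tick uses with a Delay to repeat the 2D gravity-flip sound roughly every second.
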(event OnComponentBeginOverlap(Box)
  (params (OverlappedComponent :type Primitive%20Component%20Object%20Reference) (OtherActor :type Actor%20Object%20Reference) (OtherComp :type Primitive%20Component%20Object%20Reference) (OtherBodyIndex :type Integer) (bFromSweep :type Boolean) (SweepResult :type Hit%20Result%20Structure%20%28by%20ref%29))
  (bind _asbp_htk_character (Utilities|Casting|CastToBP_HtkCharacter OtherActor))
  (Class|CharacterMovementComponent|SetGravityDirection (Variables|/Script/Engine.Character|GetCharacterMovement _asbp_htk_character) (Math|Vector|MakeVector 0.0 0.0 1.0))
  (Default|FlipControlls _asbp_htk_character)
  (Variables|Default|SetPlaySound true))

(event OnComponentEndOverlap(Box)
  (params (OverlappedComponent :type Primitive%20Component%20Object%20Reference) (OtherActor :type Actor%20Object%20Reference) (OtherComp :type Primitive%20Component%20Object%20Reference) (OtherBodyIndex :type Integer))
  (bind _asbp_htk_character (Utilities|Casting|CastToBP_HtkCharacter OtherActor))
  (Class|CharacterMovementComponent|SetGravityDirection (Variables|/Script/Engine.Character|GetCharacterMovement _asbp_htk_character) (Math|Vector|MakeVector 0.0 0.0 -1.0))
  (Default|FlipControllsBack _asbp_htk_character)
  (Variables|Default|SetPlaySound false))

(event EventTick
  (params (DeltaSeconds :type Float%20%28single-precision%29))
  (if (Variables|Default|GetPlaySound)
    (Utilities|FlowControl|Delay 1.0)
    (Audio|PlaySound2D "/Game/SFX/gravity_flip.gravity_flip" 0.2 1.0 0.0 0 0)))

(event EventBeginPlay
  (Variables|Default|SetCharacter (Game|GetPlayerCharacter 0)))

(fn ConstructionScript)