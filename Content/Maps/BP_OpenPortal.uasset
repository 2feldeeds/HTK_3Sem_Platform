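; Interactable portal Blueprint that starts a countdown when Interact fires.
; Interact plays a button click, sets TimeLeft through OpenPortalProgress and enables the countdown, which Tick decrements by delta time and prints.
; A separate Close event stops and zeroes the expired timer, but nothing in this graph calls it, and no portal opening logic is present.
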(event Custom|OpenPortalProgress
  (Variables|Default|SetTimeLeft 2e+02))

(event Custom|Close
  (if (<= (Variables|Default|GetTimeLeft) 0.0)
    (Variables|Default|SetStartCountDown false)
    (Variables|Default|SetTimeLeft 0.0)))

(event EventBeginPlay)

(event Collision|EventActorBeginOverlap
  (params (OtherActor :type Actor%20Object%20Reference)))

(event EventInteract
  (Audio|PlaySound2D "/Engine/VREditor/Sounds/UI/Click_on_Button.Click_on_Button" 1.0 1.0 0.0 0 0)
  (CallFunction|OpenPortalProgress)
  (Variables|Default|SetStartCountDown true))

(event EventTick
  (params (DeltaSeconds :type Float%20%28single-precision%29))
  (if (Variables|Default|GetStartCountDown)
    (Variables|Default|SetTimeLeft (- (Variables|Default|GetTimeLeft) DeltaSeconds))
    (Development|PrintString (Utilities|String|ToString(Float) (Variables|Default|GetTimeLeft)))))

(fn ConstructionScript)