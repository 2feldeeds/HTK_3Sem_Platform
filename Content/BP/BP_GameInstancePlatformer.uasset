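; Platformer game instance that holds the player's spawn transform and volume settings, backed by a BP_SaveGame object.
; Init loads or creates the save and applies its volumes through sound mix class overrides, but never copies the saved spawn into the instance.
; Shutdown writes the spawn to Platformsavegame.
; SetVolumeValue saves the same object to a separate VolumeValues slot, which Init does not read, without reapplying the mix.
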(event EventInit
  (bind _returnvalue (SaveGame|LoadGamefromSlot (Variables|Default|Getplatformsavegame)))
  (bind _asbp_save_game (Utilities|Casting|CastToBP_SaveGame _returnvalue)
    (:then
      (bind _output_get (Variables|Default|SetSave%20Game _asbp_save_game))
      (Variables|/Game/BP/BP_SaveGame.BP_SaveGame_C|SetHasValidSpawnTransform _output_get (Variables|/Game/BP/BP_SaveGame.BP_SaveGame_C|GetHasValidSpawnTransform _output_get))
      (Variables|/Game/BP/BP_SaveGame.BP_SaveGame_C|SetPlayerSpawn _output_get (Variables|Default|GetPlayerSpawnTransform)))
    (:CastFailed
      (bind _returnvalue_2 (SaveGame|CreateSaveGameObject "/Game/BP/BP_SaveGame.BP_SaveGame_C"))
      (Variables|Default|SetSave%20Game _returnvalue_2)))
  (CallFunction|ApplyVolumeSettings))

(event EventShutdown
  (bind _save_game (Variables|Default|GetSave%20Game))
  (Variables|/Game/BP/BP_SaveGame.BP_SaveGame_C|SetHasValidSpawnTransform _save_game (Variables|Default|GetHasPlayerSpawnTransform))
  (Variables|/Game/BP/BP_SaveGame.BP_SaveGame_C|SetPlayerSpawn _save_game (Variables|Default|GetPlayerSpawnTransform))
  (SaveGame|SaveGametoSlot _save_game (Variables|Default|Getplatformsavegame)))

(fn SetPlayerSpawnTransform
  (params (PlayerSpawnTransform :type Transform))
  (Variables|Default|SetPlayerSpawnTransform PlayerSpawnTransform)
  (Variables|Default|SetHasPlayerSpawnTransform true))

(fn TryGetPlayerSpawnTransform
  (return (Variables|Default|GetPlayerSpawnTransform) (Variables|Default|GetHasPlayerSpawnTransform)))

(fn SetVolumeValue
  (params (Volume_Masteer :type Float%20%28double-precision%29) (Volume_Music :type Float%20%28double-precision%29) (Volume_Sfx :type Float%20%28double-precision%29))
  (bind _save_game (Variables|Default|GetSave%20Game))
  (Variables|/Game/BP/BP_SaveGame.BP_SaveGame_C|SetVolume_Masteer _save_game Volume_Masteer)
  (Variables|/Game/BP/BP_SaveGame.BP_SaveGame_C|SetVolume_Music _save_game Volume_Music)
  (Variables|/Game/BP/BP_SaveGame.BP_SaveGame_C|SetVolume_Sfx _save_game Volume_Sfx)
  (SaveGame|SaveGametoSlot _save_game (Variables|Default|GetVolumeValues)))

(fn ApplyVolumeSettings
  (bind _save_game (Variables|Default|GetSave%20Game))
  (Audio|SetSoundMixClassOverride "/Game/SFX/SoundMix_Htk.SoundMix_Htk" "/Game/SFX/Master_Htk.Master_Htk" (Variables|/Game/BP/BP_SaveGame.BP_SaveGame_C|GetVolume_Masteer _save_game) 1.0 1.0 true)
  (Audio|SetSoundMixClassOverride "/Game/SFX/SoundMix_Htk.SoundMix_Htk" "/Game/SFX/Music_Htk.Music_Htk" (Variables|/Game/BP/BP_SaveGame.BP_SaveGame_C|GetVolume_Music _save_game) 1.0 1.0 true)
  (Audio|SetSoundMixClassOverride "/Game/SFX/SoundMix_Htk.SoundMix_Htk" "/Game/SFX/SFX_Htk.SFX_Htk" (Variables|/Game/BP/BP_SaveGame.BP_SaveGame_C|GetVolume_Sfx _save_game) 1.0 1.0 true))