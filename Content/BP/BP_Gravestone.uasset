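; Gravestone actor that randomizes its own look so placed instances vary in height, tilt, size and mesh.
; On BeginPlay, four custom events give its mesh component a random relative Z offset, X/Y tilt, uniform scale and a mesh picked from an array.
; Offset and tilt limits and the upper scale bound come from variables.
; The construction script is empty, so the variation is rolled at runtime only.
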(event Custom|Z-%20Random
  (bind _maxheightoffset (Variables|Default|GetMaxHeightOffset))
  ;[0.8615 0.02334 0 0.5] Zufällige Offset (Z-Achse)
  (Transformation|SetRelativeLocation (Variables|Default|GetCube) (Math|Vector|MakeVector 0.0 0.0 (Math|Random|RandomFloatinRange (* -1.0 _maxheightoffset) _maxheightoffset)) false false))

(event Custom|X-,Y-%20Rotation
  (bind _neigungy (Variables|Default|GetNeigungY))
  (bind _neigungx (Variables|Default|GetNeigungX))
  ;[0.06294 0.04799 0.15 0.5] X-, Y- Rotation
  (Transformation|SetRelativeRotation (Variables|Default|GetCube) (Math|Rotator|MakeRotator (Math|Random|RandomFloatinRange (* -1.0 _neigungx) _neigungx) (Math|Random|RandomFloatinRange (* -1.0 _neigungy) _neigungy) 0.0) false false))

(event Custom|Random%20Scale
  (bind _randomscale (Variables|Default|GetRandomScale))
  ;[0.1016 0.749 0.1371 0.5] Zufällige Größe 20%
  (Transformation|SetRelativeScale3D (Variables|Default|GetCube) (Math|Conversions|ToVector(Float) (Math|Random|RandomFloatinRange (- _randomscale 0.2) _randomscale))))

(event Custom|Random%20Mesh
  ;[0.5565 0.9031 0 0.5] Asign random mesh( 3 posible variation)
  (Components|StaticMesh|SetStaticMesh (Variables|Default|GetCube) (.OutItem (Utilities|Array|Random (Variables|Default|GetMeshes)))))

(event EventBeginPlay
  (CallFunction|Z-Random)
  (CallFunction|X-,Y-Rotation)
  (CallFunction|RandomScale)
  (CallFunction|RandomMesh))

(event Collision|EventActorBeginOverlap
  (params (OtherActor :type Actor%20Object%20Reference)))

(event EventTick
  (params (DeltaSeconds :type Float%20%28single-precision%29)))

(fn ConstructionScript)