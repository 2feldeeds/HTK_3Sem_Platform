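; BP_StoneRune is a stone rune actor that lights up when a BP_HtkCharacter enters its sphere and fades when the character leaves.
; A dynamic material instance created on the cube at BeginPlay receives its EmissiveStrength from a timeline curve scaled by a strength variable.
; Overlap begin plays the timeline and overlap end reverses it.
; IsOn becomes true whenever the timeline finishes, and nothing here clears it.
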(event OnComponentBeginOverlap(Sphere)
  (params (OverlappedComponent :type Primitive%20Component%20Object%20Reference) (OtherActor :type Actor%20Object%20Reference) (OtherComp :type Primitive%20Component%20Object%20Reference) (OtherBodyIndex :type Integer) (bFromSweep :type Boolean) (SweepResult :type Hit%20Result%20Structure%20%28by%20ref%29))
  (Utilities|Casting|CastToBP_HtkCharacter OtherActor)
  (bind _emmisive (Timeline|Timeline Play)
    (:Update
      (Rendering|Material|SetScalarParameterValue (Variables|Default|GetMID) "EmissiveStrength" (* _emmisive (Variables|Default|GetEmmisiveStrengh)) :!class /Script/Engine.MaterialInstanceDynamic))
    (:Finished
      (Variables|Default|SetIsOn true))))

(event OnComponentEndOverlap(Sphere)
  (params (OverlappedComponent :type Primitive%20Component%20Object%20Reference) (OtherActor :type Actor%20Object%20Reference) (OtherComp :type Primitive%20Component%20Object%20Reference) (OtherBodyIndex :type Integer))
  (Utilities|Casting|CastToBP_HtkCharacter OtherActor)
  (bind _emmisive (Timeline|Timeline Reverse)
    (:Update
      (Rendering|Material|SetScalarParameterValue (Variables|Default|GetMID) "EmissiveStrength" (* _emmisive (Variables|Default|GetEmmisiveStrengh)) :!class /Script/Engine.MaterialInstanceDynamic))
    (:Finished
      (Variables|Default|SetIsOn true))))

(event EventBeginPlay
  (bind _returnvalue (Rendering|Material|CreateDynamicMaterialInstance (Variables|Default|GetCube) 0 0 "None" :!class /Script/Engine.PrimitiveComponent))
  (Variables|Default|SetMID _returnvalue))

(fn ConstructionScript)