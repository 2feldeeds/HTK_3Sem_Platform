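; BP_KillZone is a gas hazard volume that repeatedly damages the player while a BP_HtkCharacter is inside its box.
; Box overlap begin and end set an IsInGas flag, with entry triggering damage immediately.
; A custom Applydamage event re-calls itself after a short delay while the flag holds, always damaging player pawn 0 rather than the overlapping actor.
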(event OnComponentBeginOverlap(Box)
  (params (OverlappedComponent :type Primitive%20Component%20Object%20Reference) (OtherActor :type Actor%20Object%20Reference) (OtherComp :type Primitive%20Component%20Object%20Reference) (OtherBodyIndex :type Integer) (bFromSweep :type Boolean) (SweepResult :type Hit%20Result%20Structure%20%28by%20ref%29))
  (Utilities|Casting|CastToBP_HtkCharacter OtherActor)
  (Variables|Default|SetIsInGas true)
  (CallFunction|ApplyDamage))

(event OnComponentEndOverlap(Box)
  (params (OverlappedComponent :type Primitive%20Component%20Object%20Reference) (OtherActor :type Actor%20Object%20Reference) (OtherComp :type Primitive%20Component%20Object%20Reference) (OtherBodyIndex :type Integer))
  (Utilities|Casting|CastToBP_HtkCharacter OtherActor)
  (Variables|Default|SetIsInGas false))

(event Custom|Apply%20damage
  (if (Variables|Default|GetIsInGas)
    (Game|Damage|ApplyDamage (Game|Player|GetPlayerPawn 0) 25.0 0 0)
    (Utilities|FlowControl|Delay 1.0)
    (CallFunction|ApplyDamage)))

(fn ConstructionScript)