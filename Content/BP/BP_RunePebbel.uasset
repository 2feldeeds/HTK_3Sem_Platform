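; BP_RunePebbel is a rune pebble actor that glows brighter as the player approaches.
; BeginPlay creates a dynamic material instance on the Cube mesh, and Tick drives its EmissiveStrength from the clamped, inverted distance to the player pawn relative to MaxGlowDis.
; A separate ApplyRuneRotation event gives the Cube a random relative yaw and is not called within this graph.
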(event Custom|ApplyRuneRotation
  (Transformation|SetRelativeRotation (Variables|Default|GetCube) (Math|Rotator|MakeRotator 0.0 0.0 (Math|Random|RandomFloatinRange 0.0 3.6e+02)) false false))

(event EventBeginPlay
  (bind _returnvalue (Rendering|Material|CreateDynamicMaterialInstance (Variables|Default|GetCube) 0 0 "None" :!class /Script/Engine.PrimitiveComponent))
  (Variables|Default|SetMID _returnvalue))

(event EventTick
  (params (DeltaSeconds :type Float%20%28single-precision%29))
  (Rendering|Material|SetScalarParameterValue (Variables|Default|GetMID) "EmissiveStrength" (* (- 1.0 (Math|Float|Clamp(Float) (/ (Math|Vector|Distance(Vector) (Transformation|GetActorLocation (Game|Player|GetPlayerPawn 0)) (Transformation|GetActorLocation)) (Variables|Default|GetMaxGlowDis)))) 1e+01) :!class /Script/Engine.MaterialInstanceDynamic))

(fn ConstructionScript)