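; A practice actor whose mesh drifts steadily upward while its point light changes color and brightness at random.
; Tick moves the mesh at a delta-time-scaled speed, then a Delay throttles RandomizeLight to about once a second, picking a random color and an intensity between two variables.
; BeginPlay calls ModifyMesh, but that function's transform, mesh-swap and print nodes are disconnected, so it does nothing.
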(event Custom|Randomize%20light
  (bind _pointlight (Variables|Default|GetPointLight))
  ;[0.04933 0.15 0.04172 0.5] Custom Event Color
  (Rendering|Components|Light|SetLightColor _pointlight (Utilities|Struct|MakeLinearColor (Math|Random|RandomFloat) (Math|Random|RandomFloat) (Math|Random|RandomFloat) 1.0) false)
  (Rendering|Components|Light|SetIntensity _pointlight (Math|Random|RandomFloatinRange (Variables|Default|GetLightIntensetyMIn) (Variables|Default|GetLightIntesetyMax))))

(event EventBeginPlay
  (|ModifyMesh))

(event Collision|EventActorBeginOverlap
  (params (OtherActor :type Actor%20Object%20Reference))
  ;[0.15 0.07658 0.02883 0.5] Trigger and Collision
)

(event Collision|EventHit
  (params (MyComp :type Primitive%20Component%20Object%20Reference) (Other :type Actor%20Object%20Reference) (OtherComp :type Primitive%20Component%20Object%20Reference) (bSelfMoved :type Boolean) (HitLocation :type Vector :default "0, 0, 0") (HitNormal :type Vector :default "0, 0, 0") (NormalImpulse :type Vector :default "0, 0, 0") (Hit :type Hit%20Result%20Structure%20%28by%20ref%29))
  ;[0.15 0.07658 0.02883 0.5] Trigger and Collision
)

(event EventTick
  (params (DeltaSeconds :type Float%20%28single-precision%29))
  (Transformation|AddWorldOffset (Variables|Default|GetMesh) (* "0.000000,0.000000,20.000000" DeltaSeconds) false false)
  (Utilities|FlowControl|Delay 1.0)
  (CallFunction|RandomizeLight))

(fn ConstructionScript)