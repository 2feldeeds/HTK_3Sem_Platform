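; Gate actor that opens when three linked rune stones are all switched on.
; Tick polls the IsOn flag of RuneStone00, RuneStone01 and RuneStone02 every frame and calls Open while all three are set.
; Open plays a timeline that moves the Scene component along relative Z by the track value scaled by DistanceZ.
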(event Custom|Open
  (bind _newtrack_0 (Timeline|Timeline Play)
    (:Update
      (Transformation|SetRelativeLocation (Variables|Default|GetScene) (Math|Vector|MakeVector 0.0 0.0 (* _newtrack_0 (Variables|Default|GetDistanceZ))) false false))))

(event EventTick
  (params (DeltaSeconds :type Float%20%28single-precision%29))
  (if (Math|Boolean|ANDBoolean (Variables|/Game/BP/BP_StoneRune.BP_StoneRune_C|GetIsOn (Variables|Default|GetRune_Stone0_0)) (Variables|/Game/BP/BP_StoneRune.BP_StoneRune_C|GetIsOn (Variables|Default|GetRune_Stone0_1)) (Variables|/Game/BP/BP_StoneRune.BP_StoneRune_C|GetIsOn (Variables|Default|GetRune_Stone0_2)))
    (CallFunction|Open)))

(fn ConstructionScript)