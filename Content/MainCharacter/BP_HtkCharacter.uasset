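; Player character with yoyo weapon: camera-relative movement, run, jump, interaction, random-combo punches, held heavy punch and charged yoyo throw.
; Tick turns it toward the nearest enemy when close or aiming, computes fall damage from velocity, and disables input while airborne or IsDead, which doubles as an action lock.
; Damage flashes the skin material; death fades the camera and teleports to the GameInstance spawn.
; Sphere-trace functions detect hits, with weapon hits launching enemies.
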(event Custom|Falling
  (bind _charactermovement (Variables|Character|GetCharacterMovement))
  (bind _velocity (Variables|/Script/Engine.MovementComponent|GetVelocity _charactermovement))
  (bind _returnvalue (Math|Float|Absolute(Float) (.z _velocity)))
  ;[0.15 0.01516 0.01516 0.5] Fall Damage
  (if (AI|Components|NavMovement|IsFalling (Variables|Character|GetCharacterMovement))
    (if (> _returnvalue 9e+02)
      (Variables|Default|SetFallDamage (Math|Float|Power (/ (/ _returnvalue 85.0) 8.5) (+ (/ _returnvalue 3e+03) 2.0))))))

(event Custom|EquipWeapon
  ;[0.15 0.1408 0 0.5] Punch
  (Transformation|AttachComponentToComponent (Variables|Default|GetWeapon) (Variables|Character|GetMesh) "Weapon" "KeepRelative" "KeepRelative" "KeepRelative" true))

(event Custom|Respawn
  (bind _returnvalue (Game|GetPlayerCameraManager 0))
  ;[0.06157 0.15 0.04203 0.5] Health & Death
  (Variables|Default|SetIsDead true)
  (Utilities|FlowControl|DoOnce false :!label _label
    (:Completed
      (Animation|Montage|PlayMontage (Variables|Character|GetMesh) "/Game/MainCharacter/Animation/AnimationMontage/AM_Death.AM_Death"
        (:then
          (CameraFades|StartCameraFade :self _returnvalue :ToAlpha 1.0 :Duration 1.0 :bHoldWhenFinished true)
          (Utilities|FlowControl|Delay 1.0)
          (CallFunction|TeleporttoSpawn)
          (Variables|Default|SetCurrentHealth 1e+02)
          (Utilities|FlowControl|Delay 1.0)
          (CameraFades|StartCameraFade :self _returnvalue :FromAlpha 1.0 :Duration 1.0 :bHoldWhenFinished true)
          (Animation|Montage|PlayMontage (Variables|Character|GetMesh) 0
            (:then
              (Variables|Default|SetIsDead false)
              (goto _label Reset))))))))

(event Custom|Update%20Attack%20type
  ;[0.15 0.1408 0 0.5] Punch
  (bind _output_get (Variables|Default|SetAttackType (Math|Random|RandomInteger (Utilities|Array|Length (Variables|Default|GetCombo))))))

(event Custom|Hurt
  (bind _mesh (Variables|Character|GetMesh))
  (Rendering|Material|SetMaterial _mesh 0 "/Game/MainCharacter/Material/M_YoyoDamage.M_YoyoDamage")
  (Utilities|FlowControl|Delay 1.0)
  (Rendering|Material|SetMaterial _mesh 0 "/Game/MainCharacter/Material/M_YoyoSkin.M_YoyoSkin"))

(event Custom|Find%20Actor
  ;[0.05226 0.04323 0.15 0.5] Look At Enemy
  (bind _outactors (Actor|GetAllActorsOfClass "/Game/Enemy/BP_EnemyDefault.BP_EnemyDefault_C"))
  (if (or (<= (.Distance (Actor|FindNearestActor (Transformation|GetActorLocation) _outactors)) 3e+02) (Variables|Default|GetIsAiming))
    (Variables|Default|SetTarget (.ReturnValue (Actor|FindNearestActor (Transformation|GetActorLocation) _outactors)))
    (Transformation|SetActorRotation self (Math|Interpolation|RInterpTo (Transformation|GetActorRotation) (Math|Rotator|FindLookatRotation (Transformation|GetActorLocation) (Transformation|GetActorLocation (Variables|Default|GetTarget))) (Utilities|Time|GetWorldDeltaSeconds) (Variables|Default|GetInterp%20Speed)))))

(event Custom|WeaponSpin
  ;[0.15 0.1408 0 0.5] Punch
  (Transformation|SetRelativeRotation (Variables|Default|GetSpiningPivot) "0.000000,100.000000,0.000000" false false))

(event Custom|Time
  ;[0.15 0.15 0.15 0.5] Update
  (Variables|Default|SetDefaultPunchTime (+ (Utilities|Time|GetWorldDeltaSeconds) (Variables|Default|GetDefaultPunchTime))))

(event Custom|Hide%20Weapon
  ;[0.15 0.1408 0 0.5] Punch
  (Rendering|SetVisibility (Variables|Default|GetWeaponNoRope) false false)
  (Rendering|SetVisibility (Variables|Default|GetCable) false false)
  (Rendering|SetVisibility (Variables|Default|GetWeapon) false false))

(event Custom|Blinking
  (bind _mesh (Variables|Character|GetMesh))
  (Rendering|Material|SetMaterial _mesh 0 "/Game/MainCharacter/Material/M_YoyoSkin.M_YoyoSkin")
  (Utilities|FlowControl|Delay (Math|Random|RandomFloatinRange 1.0 5.0))
  (Rendering|Material|SetMaterial _mesh 0 "/Game/MainCharacter/Material/M_YoyoBlink.M_YoyoBlink")
  (Utilities|FlowControl|Delay 0.2)
  (CallFunction|Blinking))

(event Custom|HitReact
  ;[0.05226 0.04323 0.15 0.5] Look At Enemy
  (if (Variables|Default|GetGetHit)
    ;[0.15 0.15 0.15 0.5] Reaction When Hit
    (Utilities|FlowControl|DoOnce false :!label _label
      (:Completed
        (CallFunction|EquipWeapon)
        (Animation|Montage|PlayMontage (Variables|Character|GetMesh) "/Game/MainCharacter/Animation/AnimationMontage/AM_Damaged.AM_Damaged"
          (:then
            (Game|Damage|ApplyDamage self 2e+01 0 0)
            (Utilities|FlowControl|DoOnce false :!label _label_2
              (:Completed
                (Audio|PlaySound2D "/Game/SFX/Punch_3.Punch_3" 1.0 1.0 0.0 0 0)
                (Utilities|FlowControl|Delay 0.2)
                (goto _label_2 Reset))))
          (:OnCompleted
            (goto _label Reset)))))))

(event Custom|IncreasHealth
  (params (New%20Health :type Float%20%28double-precision%29))
  ;[0.06157 0.15 0.04203 0.5] Health & Death
  (Variables|Default|SetCurrentHealth (+ (Variables|Default|GetCurrentHealth) New%20Health))
  (if (>= (Variables|Default|GetCurrentHealth) 1e+02)
    (Variables|Default|SetCurrentHealth 1e+02)))

(event Custom|InsideSpaceShip
  (Transformation|SetRelativeLocation (Variables|Collision|GetCapsuleComponent) (Transformation|GetActorLocation (Variables|Default|GetInsideTheSpaceShip)) false false))

(event Custom|OutsideSpaceShip
  (Transformation|SetRelativeLocation (Variables|Collision|GetCapsuleComponent) (Transformation|GetActorLocation (Variables|Default|GetOutsideTheSpaceSHip)) false false))

(event Custom|DisableInputs
  ;[0.15 0.15 0.15 0.5] Disable Input
  (if (or (not (AI|Components|NavMovement|IsMovingonGround (Variables|Character|GetCharacterMovement))) (Variables|Default|GetIsDead))
    (Input|DisableInput 0)
    (else
      (Input|EnableInput 0))))

(event Custom|UnarmWeapon
  ;[0.15 0.1408 0 0.5] Punch
  (Transformation|AttachComponentToComponent (Variables|Default|GetWeapon) (Variables|Character|GetMesh) "WeaponHolder" "KeepRelative" "KeepRelative" "KeepRelative" true))

(event Custom|VisibilityWapon
  ;[0.15 0.1408 0 0.5] Punch
  (Rendering|SetVisibility (Variables|Default|GetWeapon) true false)
  (Rendering|SetVisibility (Variables|Default|GetRope) false false))

(event Input|EnhancedActionEvents|EnhancedInputActionIA_Move
  (params (ActionValue :type Vector%202D%20Structure) (ElapsedSeconds :type Float%20%28double-precision%29) (TriggeredSeconds :type Float%20%28double-precision%29) (InputAction :type Input%20Action%20Object%20Reference :default "/Game/Input/Action/IA_Move.IA_Move"))
  ;[0.15 0.05975 0.05452 0.5] Inputs
  (if true
    (CallFunction|CameraDirection (.x ActionValue) (.y ActionValue))))

(event Input|EnhancedActionEvents|EnhancedInputActionIA_Interact
  (params (ActionValue :type Boolean) (ElapsedSeconds :type Float%20%28double-precision%29) (TriggeredSeconds :type Float%20%28double-precision%29) (InputAction :type Input%20Action%20Object%20Reference :default "/Game/Input/Action/IA_Interact.IA_Interact"))
  (bind _interactionsphere (Variables|Default|GetInteractionSphere))
  ;[0.04243 0.03566 0.15 0.5] Interaction
  (bind _outactors (Collision|SphereOverlapActors (Transformation|GetWorldLocation _interactionsphere) (Components|Sphere|GetScaledSphereRadius _interactionsphere) (Utilities|Array|MakeArray "ObjectTypeQuery3" "ObjectTypeQuery1" "ObjectTypeQuery2") 0 (Utilities|Array|MakeArray self)))
  (for _array_element _outactors
    (if (Utilities|DoesObjectImplementInterface _array_element "/Game/Interaction/IInteractable.IInteractable_C")
      (Class|IInteractable|Interact(Message) _array_element))))

(event Input|EnhancedActionEvents|EnhancedInputActionIA_Look
  (params (ActionValue :type Vector%202D%20Structure) (ElapsedSeconds :type Float%20%28double-precision%29) (TriggeredSeconds :type Float%20%28double-precision%29) (InputAction :type Input%20Action%20Object%20Reference :default "/Game/Input/Action/IA_Look.IA_Look"))
  ;[0.15 0.05975 0.05452 0.5] Inputs
  (Pawn|Input|AddControllerYawInput (.x ActionValue))
  (Pawn|Input|AddControllerPitchInput (.y ActionValue)))

(event Input|EnhancedActionEvents|EnhancedInputActionIA_Jump
  (params (ActionValue :type Boolean) (ElapsedSeconds :type Float%20%28double-precision%29) (TriggeredSeconds :type Float%20%28double-precision%29) (InputAction :type Input%20Action%20Object%20Reference :default "/Game/Input/Action/IA_Jump.IA_Jump"))
  ;[0.15 0.05975 0.05452 0.5] Inputs
  (:Started
    (Character|Jump)
    (if (AI|Components|NavMovement|IsMovingonGround (Variables|Character|GetCharacterMovement))
      (Audio|PlaySound2D "/Game/SFX/Jump.Jump" 1.0 1.0 0.0 0 0)))
  (:Completed
    (Character|StopJumping)))

(event Input|EnhancedActionEvents|EnhancedInputActionIA_Run
  (params (ActionValue :type Boolean) (ElapsedSeconds :type Float%20%28double-precision%29) (TriggeredSeconds :type Float%20%28double-precision%29) (InputAction :type Input%20Action%20Object%20Reference :default "/Game/Input/Action/IA_Run.IA_Run"))
  (bind _charactermovement (Variables|Character|GetCharacterMovement))
  ;[0.15 0.05975 0.05452 0.5] Inputs
  (:Triggered
    (Variables|/Script/Engine.CharacterMovementComponent|SetMaxWalkSpeed _charactermovement 8e+02))
  (:Completed
    (Variables|/Script/Engine.CharacterMovementComponent|SetMaxWalkSpeed _charactermovement 2.5e+02)))

(event Input|EnhancedActionEvents|EnhancedInputActionIA_Pause
  (params (ActionValue :type Boolean) (ElapsedSeconds :type Float%20%28double-precision%29) (TriggeredSeconds :type Float%20%28double-precision%29) (InputAction :type Input%20Action%20Object%20Reference :default "/Game/Input/Action/IA_Pause.IA_Pause"))
  ;[0.15 0.05975 0.05452 0.5] Inputs
  (bind _asbp_hud (Utilities|Casting|CastToBP_HUD (HUD|GetHUD (Game|GetPlayerController 0))))
  (Default|Pause _asbp_hud))

(event Input|EnhancedActionEvents|EnhancedInputActionIA_Punch
  (params (ActionValue :type Boolean) (ElapsedSeconds :type Float%20%28double-precision%29) (TriggeredSeconds :type Float%20%28double-precision%29) (InputAction :type Input%20Action%20Object%20Reference :default "/Game/Input/Action/IA_Punch.IA_Punch"))
  ;[0.15 0.1408 0 0.5] Punch
  (if (> (Variables|Default|GetDefaultPunchTime) 1.02)
    (Animation|Montage|PlayMontage (Variables|Character|GetMesh) (Utilities|Array|Get(acopy) (Variables|Default|GetCombo) (stale Custom|Update%20Attack%20type _output_get)) 1.0 0.0 "PunchStart"
      (:then
        (Variables|Default|SetDefaultPunchTime 0.0)))))

(event Input|EnhancedActionEvents|EnhancedInputActionIA_HardPunch
  (params (ActionValue :type Boolean) (ElapsedSeconds :type Float%20%28double-precision%29) (TriggeredSeconds :type Float%20%28double-precision%29) (InputAction :type Input%20Action%20Object%20Reference :default "/Game/Input/Action/IA_HardPunch.IA_HardPunch"))
  ;[0.15 0.1408 0 0.5] Punch
  (:Triggered
    (Variables|Default|SetHardPunch (+ (Utilities|Time|GetWorldDeltaSeconds) (Variables|Default|GetHardPunch)))
    (if (>= (Variables|Default|GetHardPunch) 2.0)
      (Variables|Default|SetIsDead true)
      (Animation|Montage|PlayMontage (Variables|Character|GetMesh) "/Game/MainCharacter/Animation/AnimationMontage/AM_HardPunch.AM_HardPunch"
        (:then
          (Variables|Default|SetHardPunch 0.0)
          (Utilities|FlowControl|Delay 2.0)
          (Variables|Default|SetIsDead false)))))
  (:Completed
    (Variables|Default|SetHardPunch 0.0)))

(event Input|EnhancedActionEvents|EnhancedInputActionIA_Charge
  (params (ActionValue :type Boolean) (ElapsedSeconds :type Float%20%28double-precision%29) (TriggeredSeconds :type Float%20%28double-precision%29) (InputAction :type Input%20Action%20Object%20Reference :default "/Game/Input/Action/IA_Charge.IA_Charge"))
  (bind _mesh (Variables|Character|GetMesh))
  (bind _trowdirection (Variables|Default|GetTrowDirection))
  (bind _returnvalue (Transformation|GetWorldTransform _trowdirection))
  ;[0.15 0.1408 0 0.5] Punch
  (:Triggered
    (Variables|Default|SetTrowWeaponProgress (+ (Utilities|Time|GetWorldDeltaSeconds) (Variables|Default|GetTrowWeaponProgress)))
    (Animation|Montage|PlayMontage _mesh "/Game/MainCharacter/Animation/AnimationMontage/AM_Aim.AM_Aim"
      (:then
        (Variables|Default|SetIsAiming true)
        (Rendering|SetVisibility (Variables|Default|GetWeaponNoRope) true false)
        (Rendering|SetVisibility (Variables|Default|GetCable) true false)
        (Rendering|SetVisibility (Variables|Default|GetRope) true false)
        (if (>= (Variables|Default|GetTrowWeaponProgress) 2.0)
          (Variables|Default|SetTrowWeaponProgress 0.0)
          (Animation|Montage|PlayMontage _mesh "/Game/MainCharacter/Animation/AnimationMontage/AM_Launch.AM_Launch"
            (:then
              (Variables|Default|SetIsDead true)
              (Utilities|FlowControl|Delay 0.24)
              (Variables|Default|SetIsAiming false)
              (Game|SpawnActorfromClass "/Game/MainCharacter/BP_YoyoTrowable.BP_YoyoTrowable_C" (Math|Transform|MakeTransform (.location _returnvalue) (.rotation _returnvalue) "1.000000,1.000000,1.000000") "Undefined" "MultiplyWithRoot" 0 0)
              (CallFunction|HideWeapon)))
          (else
            (CallFunction|HideWeapon)
            (CallFunction|VisibilityWapon)
            (Animation|Montage|PlayMontage _mesh "/Game/MainCharacter/Animation/AnimationMontage/AM_Launch.AM_Launch"))))))
  (:Completed
    (Variables|Default|SetTrowWeaponProgress 0.0)))

(event Game|Damage|EventAnyDamage
  (params (Damage :type Float%20%28single-precision%29) (DamageType :type Damage%20Type%20Object%20Reference) (InstigatedBy :type Controller%20Object%20Reference) (DamageCauser :type Actor%20Object%20Reference))
  ;[0.06157 0.15 0.04203 0.5] Health & Death
  (CallFunction|Hurt)
  (bind _output_get (Variables|Default|SetCurrentHealth (Math|Float|Clamp(Float) (- (Variables|Default|GetCurrentHealth) Damage) 0.0 1e+02)))
  (if (<= _output_get 0.0)
    (Rendering|Material|SetMaterial (Variables|Character|GetMesh) 0 "/Game/MainCharacter/Material/M_YoyoDamage.M_YoyoDamage")
    (Animation|Montage|PlayMontage (Variables|Character|GetMesh) "/Game/MainCharacter/Animation/AnimationMontage/AM_Damaged.AM_Damaged"
      (:then
        (CallFunction|Respawn)))))

(event EventTick
  (params (DeltaSeconds :type Float%20%28single-precision%29))
  ;[0.15 0.15 0.15 0.5] Update
  (CallFunction|FindActor)
  (CallFunction|Falling)
  (CallFunction|UpdateAttackType)
  (CallFunction|Time)
  (CallFunction|DisableInputs)
  (CallFunction|WeaponSpin)
  (Development|PrintString (Utilities|String|ToString(Float) (Variables|Default|GetTrowWeaponProgress))))

(event EventBeginPlay
  ;[0.15 0.05975 0.05452 0.5] Inputs
  (CallFunction|TeleporttoSpawn)
  (Input|AddMappingContext (PlayerController|LocalPlayerSubsystems|GetEnhancedInputLocalPlayerSubsystem (Game|GetPlayerController 0)) "/Game/Input/IMC_Default.IMC_Default" 0 "(bIgnoreAllPressedKeysUntilRelease=True,bForceImmediately=False,bNotifyUserSettings=False)")
  (bind _returnvalue (UserInterface|CreateWidget "/Game/UI/Widgets/WBP_GameUI.WBP_GameUI_C"))
  (UserInterface|Viewport|AddtoViewport _returnvalue 0)
  (CallFunction|Blinking))

(event EventOnLanded
  (params (Hit :type Hit%20Result%20Structure%20%28by%20ref%29))
  ;[0.15 0.01516 0.01516 0.5] Fall Damage
  (Variables|Default|SetIsDead true)
  (Game|Damage|ApplyDamage self (Variables|Default|GetFallDamage) 0 0)
  (Audio|PlaySound2D "/Game/SFX/Landing.Landing" 1.0 1.0 0.0 0 0)
  (Utilities|FlowControl|Delay 0.5)
  (Variables|Default|SetIsDead false))

(fn ConstructionScript)

(fn CameraDirection
  (params (LocalDirection_X :type Float%20%28double-precision%29) (LocalDirection_Y :type Float%20%28double-precision%29))
  (bind _camera (Variables|Default|GetCamera))
  (bind _returnvalue (Transformation|GetWorldTransform _camera))
  (Pawn|Input|AddMovementInput (Math|Transform|TransformDirection (Math|Transform|MakeTransform (.location _returnvalue) (Math|Rotator|MakeRotator 0.0 0.0 (.yaw (.rotation _returnvalue))) (.scale _returnvalue)) (Math|Vector|MakeVector LocalDirection_X LocalDirection_Y 0.0)) 1.0 false))

(fn HitDitect
  (bind _mesh (Variables|Character|GetMesh))
  (bind _attacktype (Variables|Default|GetAttackType))
  (bind _returnvalue (Utilities|Select :Index _attacktype :Option%200 "DEF-hand_R" :Option%201 "DEF-hand_L"))
  (bind _returnvalue_2 (Transformation|GetSocketLocation _mesh _returnvalue))
  (Collision|SphereTraceForObjects _returnvalue_2 _returnvalue_2 (Components|Sphere|GetScaledSphereRadius (Variables|Default|GetRight)) (Utilities|Array|MakeArray "ObjectTypeQuery3") true 0 "ForDuration" true "(R=1.000000,G=0.000000,B=0.000000,A=1.000000)" "(R=0.000000,G=1.000000,B=0.000000,A=1.000000)" 0.1))

(fn TeleporttoSpawn
  (bind _asbp_game_instance (Utilities|Casting|CastToBP_GameInstance (Game|GetGameInstance))
    (:then
      (if (.HasPlayerSpawnTransform (Default|TryGetPlayerSpawnTransform _asbp_game_instance))
        (Transformation|SetActorLocationAndRotation (.location (.PlayerSpawnTransform (Default|TryGetPlayerSpawnTransform _asbp_game_instance))) (.rotation (.PlayerSpawnTransform (Default|TryGetPlayerSpawnTransform _asbp_game_instance))))))
    (:CastFailed
      (Development|PrintString "GameInstance"))))

(fn WeaponHit
  (bind _mesh (Variables|Character|GetMesh))
  (bind _returnvalue (Transformation|GetSocketLocation _mesh "Weapon"))
  (bind _outhit (Collision|SphereTraceForObjects _returnvalue _returnvalue (Components|Sphere|GetScaledSphereRadius (Variables|Default|GetSphere)) (Utilities|Array|MakeArray "ObjectTypeQuery3") false 0 "ForDuration" true "(R=1.000000,G=0.000000,B=0.000000,A=1.000000)" "(R=0.000000,G=1.000000,B=0.000000,A=1.000000)" 0.5))
  (bind _asbp_enemy_default (Utilities|Casting|CastToBP_EnemyDefault (.HitActor (Collision|BreakHitResult _outhit))))
  (Character|LaunchCharacter _asbp_enemy_default (* (Math|Vector|GetForwardVector (Transformation|GetWorldRotation (Variables|Collision|GetCapsuleComponent))) (* (Variables|Default|GetLaunchForce) 1e+01)) false false)
  (Default|HitReactionWeapon _asbp_enemy_default))