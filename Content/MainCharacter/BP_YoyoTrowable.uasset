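; Thrown yoyo projectile that stays tethered to the player's right hand by a cable and damages what it hits.
; Each tick it reattaches the cable and sphere-traces for pawns or static world geometry.
; The first hit stops movement, starts the return, applies damage, and makes default enemies follow the player.
; The return moves it toward the player's mesh, plays a punch montage, restores the character's weapon, and destroys the yoyo.
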(event Custom|ReturnYoyo
  (Utilities|FlowControl|DoOnce false
    (:Completed
      (bind _asbp_htk_character (Utilities|Casting|CastToBP_HtkCharacter (Game|Player|GetPlayerPawn 0)))
      (Components|MoveComponentTo (Variables|Default|GetDefaultSceneRoot) (.location (Transformation|GetWorldTransform (Variables|/Script/Engine.Character|GetMesh _asbp_htk_character))) (.rotation (Transformation|GetWorldTransform (Variables|/Script/Engine.Character|GetMesh _asbp_htk_character))) false false 0.2 false)
      (Default|UnarmWeapon _asbp_htk_character)
      (Animation|Montage|PlayMontage (Variables|/Script/Engine.Character|GetMesh _asbp_htk_character) "/Game/MainCharacter/Animation/AnimationMontage/AM_HardPunch.AM_HardPunch" 0.75 0.75
        (:then
          (Rendering|SetVisibility (Variables|Default|GetStaticMesh) false false)
          (Default|VisibilityWapon _asbp_htk_character)
          (Utilities|FlowControl|Delay 1.0)
          (Default|EquipWeapon _asbp_htk_character)
          (Variables|/Game/MainCharacter/BP_HtkCharacter.BP_HtkCharacter_C|SetIsDead _asbp_htk_character false)
          (Actor|DestroyActor))))))

(event Custom|Conect%20cable
  (Class|CableComponent|SetAttachEndto (Variables|Default|GetCable) (Game|Player|GetPlayerPawn 0) "None" "DEF-hand_R"))

(event EventTick
  (params (DeltaSeconds :type Float%20%28single-precision%29))
  (bind __ (Variables|Default|Get%20))
  (bind _returnvalue (Transformation|GetWorldLocation __))
  (CallFunction|ConectCable)
  (bind (_outhit _returnvalue_2) (Collision|SphereTraceForObjects (Transformation|GetWorldLocation __) (Math|Vector|MakeVector (+ (.x _returnvalue) 1.0) (.y _returnvalue) (.z _returnvalue)) (Components|Sphere|GetScaledSphereRadius __) (Utilities|Array|MakeArray "ObjectTypeQuery3" "ObjectTypeQuery1") false (Utilities|Array|MakeArray self (Game|Player|GetPlayerPawn 0)) "ForDuration" true "(R=1.000000,G=0.000000,B=0.000000,A=1.000000)" "(R=0.000000,G=1.000000,B=0.000000,A=1.000000)" 0.1))
  (if _returnvalue_2
    (Utilities|FlowControl|DoOnce false
      (:Completed
        (Components|Movement|StopMovementImmediately (Variables|Default|GetProjectileMovement))
        (Variables|/Script/Engine.RotatingMovementComponent|SetRotationRate (Variables|Default|GetRotatingMovement) "0, 0, 0")
        (Variables|/Script/Engine.ProjectileMovementComponent|SetProjectileGravityScale (Variables|Default|GetProjectileMovement) 0.0)
        (CallFunction|ReturnYoyo)
        (Game|Damage|ApplyDamage (.HitActor (Collision|BreakHitResult _outhit)) 75.0 0 0)
        (bind _asbp_enemy_default (Utilities|Casting|CastToBP_EnemyDefault (.HitActor (Collision|BreakHitResult _outhit))))
        (Variables|/Game/Enemy/BP_EnemyDefault.BP_EnemyDefault_C|SetisSeeingPlayer _asbp_enemy_default false)
        (Default|FollowPlayer _asbp_enemy_default)
        (Audio|PlaySound2D "/Game/SFX/Landing.Landing" 1.0 1.0 0.0 0 0)
        (Audio|PlaySound2D "/Game/SFX/Punch_2.Punch_2" 1.0 1.0 0.0 0 0)))))

(fn ConstructionScript)