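; Gun-wielding enemy that approaches the player and fires from range, overriding follow, attack and look-at events from a parent enemy.
; FollowPlayer uses a DoOnce-gated AIMoveTo to close in, then calls ShootAndAim and re-arms after a short delay.
; ShootAndAim plays an aim montage and, once OverlapTime passes a random threshold, shoots, spawning a bullet and laser particle.
; LookatPlayer smoothly turns yaw toward the player while alive and seeing them.
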(event Custom|Shoot%20And%20Aim
  (bind _bullet_direction (Variables|Default|GetBullet%20direction))
  (bind _mesh (Variables|Character|GetMesh))
  (bind _returnvalue (Transformation|GetWorldTransform _bullet_direction))
  (Animation|Montage|PlayMontage _mesh "/Game/Enemy/Animation/Enemy_Gun/AM_Aim.AM_Aim"
    (:then
      (if (> (Variables|Default|GetOverlapTime) (Math|Random|RandomFloatinRange 0.5 2.0))
        (Animation|Montage|PlayMontage _mesh "/Game/Enemy/Animation/Enemy_Gun/AM_Shoot.AM_Shoot"
          (:then
            (Transformation|SetRelativeRotation (Variables|Default|GetStaticMesh) "0.000000,120.000000,0.000000" false false)
            (Game|SpawnActorfromClass "/Game/Enemy/BP_EnemyBullet.BP_EnemyBullet_C" _returnvalue "Undefined" "MultiplyWithRoot" 0 0)
            (Game|SpawnActorfromClass "/Game/Particles/BP_LaserParticle.BP_LaserParticle_C" _returnvalue "Undefined" "MultiplyWithRoot" 0 0)
            (Variables|Default|SetOverlapTime 0.0)))))))

(event EventFollowPlayer
  (if (and (not (Variables|Default|GetIsDead)) (Variables|Default|GetisSeeingPlayer))
    (Utilities|FlowControl|DoOnce false :!label _label
      (:Completed
        (AI|AIMoveTo self "0, 0, 0" (Game|Player|GetPlayerPawn 0) 2e+03 false
          (:OnSuccess
            (Variables|Default|SetisSeeingPlayer true)
            (CallFunction|ShootandAim)
            (Utilities|FlowControl|Delay 0.2)
            (goto _label Reset)))))))

(event EventLookatPlayer
  (if (and (not (Variables|Default|GetIsDead)) (Variables|Default|GetisSeeingPlayer))
    (Transformation|SetActorRotation (Math|Rotator|MakeRotator 0.0 0.0 (.yaw (Math|Interpolation|RInterpTo (Transformation|GetActorRotation) (Math|Rotator|FindLookatRotation (Transformation|GetActorLocation) (Transformation|GetActorLocation (Game|Player|GetPlayerPawn 0))) (Utilities|Time|GetWorldDeltaSeconds) 5.0))))))

(fn ConstructionScript
  (|CallParentFunction))

(fn HitDitect
  (|CallParentFunction))