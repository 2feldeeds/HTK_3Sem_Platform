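; Default melee enemy that chases a seen player with AIMoveTo and punches on a timed cooldown.
; HitDitect sphere-traces from a spine socket to launch BP_HtkCharacter and trigger its hit reaction.
; Hit-reaction events play montages and self-apply random damage, updating a camera-facing health widget; death plays a montage, hides it and updates the HUD's defeat count.
; Tick also turns the enemy toward the player once hit, while a recursive delayed material swap creates blinking.
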(event OnSeePawn(PawnSensing)
  (params (Pawn :type Pawn%20Object%20Reference))
  ;[0.15 0.1484 0.003083 0.5] Enemy AI
  (Variables|Default|SetisSeeingPlayer true)
  (CallFunction|FollowPlayer))

(event Custom|Follow%20Player
  ;[0.15 0.1484 0.003083 0.5] Enemy AI
  (if (and (Variables|Default|GetisSeeingPlayer) (not (Variables|Default|GetIsDead)))
    (AI|AIMoveTo self "0, 0, 0" (Game|Player|GetPlayerPawn 0) 8e+01 false
      (:OnSuccess
        ;[0.15 0.09412 0.05634 0.5] Punch Animation
        (if (>= (Variables|Default|GetOverlapTime) 2.0)
          (Utilities|FlowControl|DoOnce false :!label _label
            (:Completed
              (Animation|Montage|PlayMontage (Variables|Character|GetMesh) "/Game/Enemy/Animation/AM_Punch.AM_Punch" 1.0 0.0 "Punch"
                (:then
                  (Variables|Default|SetOverlapTime 0.0))
                (:OnCompleted
                  (Pawn|Components|CharacterMovement|SetMovementMode (Variables|Character|GetCharacterMovement) "MOVE_Walking" 0 :!label _label_2)
                  (goto _label Reset))
                (:OnInterrupted
                  (Utilities|FlowControl|Delay 1.0)
                  (goto _label_2))))))))))

(event Custom|TimeOverlap
  ;[0.15 0.15 0.15 0.5] Count Time
  (Variables|Default|SetOverlapTime (+ (Utilities|Time|GetWorldDeltaSeconds) (Variables|Default|GetOverlapTime))))

(event Custom|Blinking
  (|CollapseGraph))

(event Custom|HitReactionWeapon
  ;[0.1331 0.15 0.007389 0.5] HitReact
  (if true
    (Variables|Default|SetGettingHit true)
    (Utilities|FlowControl|DoOnce false :!label _label
      (:Completed
        (Animation|Montage|PlayMontage (Variables|Character|GetMesh) "/Game/Enemy/Animation/AM_PunchWeapon.AM_PunchWeapon"
          (:then
            (Game|Damage|ApplyDamage self (Math|Random|RandomFloatinRange 6e+01 7e+01) 0 0)
            (Utilities|FlowControl|DoOnce false :!label _label_2
              (:Completed
                (Audio|PlaySound2D "/Game/SFX/Punch_cue.Punch_cue" 1.0 1.0 0.0 0 0)
                (Utilities|FlowControl|Delay 0.2)
                (goto _label_2 Reset))))
          (:OnCompleted
            (goto _label Reset)))))))

(event Custom|HitReaction
  ;[0.1331 0.15 0.007389 0.5] HitReact
  (if (and (Variables|Default|GetGettingHit) (not (Variables|Default|GetIsDead)))
    (Utilities|FlowControl|DoOnce false :!label _label
      (:Completed
        (Animation|Montage|PlayMontage (Variables|Character|GetMesh) "/Game/Enemy/Animation/AM_Punched.AM_Punched"
          (:then
            (Game|Damage|ApplyDamage self (Math|Random|RandomFloatinRange 15.0 25.0) 0 0)
            (Utilities|FlowControl|DoOnce false :!label _label_2
              (:Completed
                (Audio|PlaySound2D "/Game/SFX/Punch_cue.Punch_cue" 1.0 1.0 0.0 0 0)
                (Utilities|FlowControl|Delay 0.2)
                (goto _label_2 Reset))))
          (:OnCompleted
            (goto _label Reset)))))))

(event Custom|Look%20At%20Player
  ;[0.08236 0.1471 0.15 0.5] Look at The Target
  (if (and (not (Variables|Default|GetIsDead)) (Variables|Default|GetGettingHit))
    (Transformation|SetActorRotation (Math|Rotator|MakeRotator 0.0 0.0 (.yaw (Math|Interpolation|RInterpTo (Transformation|GetActorRotation) (Math|Rotator|FindLookatRotation (Transformation|GetActorLocation) (Transformation|GetActorLocation (Game|Player|GetPlayerPawn 0))) (Utilities|Time|GetWorldDeltaSeconds) 5.0))))))

(event Custom|CountEnemies
  ;[0.15 0 0 0.5] Dead
  (bind _asbp_hud (Utilities|Casting|CastToBP_HUD (HUD|GetHUD (Game|GetPlayerController 0))))
  (Default|EnemiesDefeated (Variables|/Game/UI/BP_HUD.BP_HUD_C|GetCollectibleWidget _asbp_hud) 1))

(event Custom|WhenIsDead
  ;[0.15 0 0 0.5] Dead
  (if (Variables|Default|GetIsDead)
    (Rendering|SetVisibility (Variables|Default|GetWidget) false false)))

(event EventBeginPlay
  ;[0.03534 0.15 0 0.5] Health
  (CallFunction|Blinking)
  (bind _aswbp_enemy_hp (Utilities|Casting|CastToWBP_EnemyHP (UserInterface|GetUserWidgetObject (Variables|Default|GetWidget))))
  (bind _output_get (Variables|Default|SetEnemyRef _aswbp_enemy_hp))
  (Variables|/Game/Enemy/WBP_EnemyHP.WBP_EnemyHP_C|SetHealth _output_get (Variables|Default|GetHealth)))

(event Game|Damage|EventAnyDamage
  (params (Damage :type Float%20%28single-precision%29) (DamageType :type Damage%20Type%20Object%20Reference) (InstigatedBy :type Controller%20Object%20Reference) (DamageCauser :type Actor%20Object%20Reference))
  ;[0.15 0.069 0.09513 0.5] TakenDamage
  (bind _output_get (Variables|Default|SetHealth (Math|Float|Clamp(Float) (- (Variables|Default|GetHealth) Damage) 0.0 1e+02)))
  (Variables|/Game/Enemy/WBP_EnemyHP.WBP_EnemyHP_C|SetHealth (Variables|Default|GetEnemyRef) _output_get)
  (if (== (Variables|Default|GetHealth) 0.0)
    (Animation|Montage|PlayMontage (Variables|Character|GetMesh) "/Game/Enemy/Animation/AM_Death.AM_Death"
      (:then
        (CallFunction|CountEnemies)
        (Variables|Default|SetIsDead true)))))

(event EventTick
  (params (DeltaSeconds :type Float%20%28single-precision%29))
  (bind _widget (Variables|Default|GetWidget))
  ;[0.15 0 0 0.5] Widget HP
  (Transformation|SetWorldRotation _widget (Math|Rotator|FindLookatRotation (Transformation|GetWorldLocation _widget) (Transformation|GetWorldLocation (Variables|/Script/Engine.PlayerCameraManager|GetTransformComponent (Game|GetPlayerCameraManager 0)))) false false)
  (CallFunction|LookatPlayer)
  (CallFunction|WhenIsDead)
  (CallFunction|TimeOverlap))

(fn ConstructionScript)

(fn HitDitect
  (bind _mesh (Variables|Character|GetMesh))
  (bind _returnvalue (Transformation|GetSocketLocation _mesh "DEF-spine_006"))
  (bind _outhit (Collision|SphereTraceForObjects _returnvalue _returnvalue (Components|Sphere|GetScaledSphereRadius (Variables|Default|GetDamage)) (Utilities|Array|MakeArray "ObjectTypeQuery3") true 0 "ForDuration" true "(R=1.000000,G=0.000000,B=0.000000,A=1.000000)" "(R=0.000000,G=1.000000,B=0.000000,A=1.000000)" 0.1))
  (bind _asbp_htk_character (Utilities|Casting|CastToBP_HtkCharacter (.HitActor (Collision|BreakHitResult _outhit))))
  (Character|LaunchCharacter _asbp_htk_character (* (Math|Vector|GetForwardVector (Transformation|GetWorldRotation (Variables|Collision|GetCapsuleComponent))) (Variables|Default|GetLaunchForce)) false false)
  (Variables|/Game/MainCharacter/BP_HtkCharacter.BP_HtkCharacter_C|SetGetHit _asbp_htk_character true)
  (Default|HitReact _asbp_htk_character))