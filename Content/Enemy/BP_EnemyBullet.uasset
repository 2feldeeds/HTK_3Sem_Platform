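; BP_EnemyBullet is an enemy projectile that damages BP_HtkCharacter on contact.
; Each Tick, a very short sphere trace at its Sphere component checks world and pawn objects, with debug drawing enabled.
; The first hit passes a DoOnce, then a successful character cast applies fixed damage and destroys the bullet.
; Any other first hit consumes the DoOnce, leaving the bullet alive but unable to deal damage.
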(event EventTick
  (params (DeltaSeconds :type Float%20%28single-precision%29))
  (bind _sphere (Variables|Default|GetSphere))
  (bind _returnvalue (Transformation|GetWorldLocation _sphere))
  (bind (_outhit _returnvalue_2) (Collision|SphereTraceForObjects (Transformation|GetWorldLocation _sphere) (Math|Vector|MakeVector (+ (.x _returnvalue) 1.0) (.y _returnvalue) (.z _returnvalue)) (Components|Sphere|GetScaledSphereRadius _sphere) (Utilities|Array|MakeArray "ObjectTypeQuery2" "ObjectTypeQuery1" "ObjectTypeQuery3") false (Utilities|Array|MakeArray 0 0) "ForDuration" true "(R=1.000000,G=0.000000,B=0.000000,A=1.000000)" "(R=0.000000,G=1.000000,B=0.000000,A=1.000000)" 0.1))
  (if _returnvalue_2
    (Utilities|FlowControl|DoOnce false
      (:Completed
        (bind _asbp_htk_character (Utilities|Casting|CastToBP_HtkCharacter (.HitActor (Collision|BreakHitResult _outhit))))
        (Game|Damage|ApplyDamage _asbp_htk_character 35.0 0 0)
        (Actor|DestroyActor)))))

(fn ConstructionScript)